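; BP_PracticeTarget is a practice target actor that shatters when it takes any damage.
; Damage hides the static mesh, disables its collision and swaps in a Chaos Geometry Collection at the same transform.
; A radial impulse with high strain then breaks the simulated collection apart.
; The first piece-removal event unbinds itself, waits for the spread of the collection's removal duration range, then destroys the actor.
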(event `self.ReceiveBeginPlay`
  (add `GeometryCollectionComponent.OnChaosRemovalEvent` (`self.GeometryCollection`) (delegate `OnPieceRemoved`)))

(event `OnPieceRemoved`
  (params (RemovalEvent :type "ChaosRemovalEvent Structure (by ref)"))
  (bind _geometrycollection (`self.GeometryCollection`))
  (bind (_removalduration_x _removalduration_y) (`KismetMathLibrary.BreakVector2D` (`GeometryCollection.RemovalDuration` (`GeometryCollectionComponent.RestCollection` _geometrycollection))))
  (remove `GeometryCollectionComponent.OnChaosRemovalEvent` _geometrycollection (delegate `OnPieceRemoved`))
  (`KismetSystemLibrary.Delay` (- _removalduration_y _removalduration_x))
  (`self.K2_DestroyActor`))

(event `self.ReceiveAnyDamage`
  (params (Damage :type "Float (single-precision)") (DamageType :type "DamageType Object Reference") (InstigatedBy :type "Controller Object Reference") (DamageCauser :type "Actor Object Reference"))
  (bind _geometrycollection (`self.GeometryCollection`))
  (bind _staticmesh (`self.StaticMesh`))
  (bind _geometrycollection_2 (`self.GeometryCollection`))
  (bind _geometrycollection_3 (`self.GeometryCollection`))
  (`SceneComponent.SetVisibility` (`self.StaticMesh`) false false)
  (`PrimitiveComponent.SetCollisionEnabled` (`self.StaticMesh`) "NoCollision")
  (`SceneComponent.SetVisibility` _geometrycollection_2 true false)
  (`SceneComponent.K2_SetWorldLocationAndRotation` _geometrycollection_2 (`SceneComponent.K2_GetComponentLocation` _staticmesh) (`SceneComponent.K2_GetComponentRotation` _staticmesh) false true)
  (`ActorComponent.Activate` _geometrycollection_3 false)
  (`PrimitiveComponent.SetSimulatePhysics` _geometrycollection_3 true)
  (`PhysicsObjectBlueprintLibrary.ApplyRadialImpulse` _geometrycollection (`SceneComponent.K2_GetComponentLocation` _geometrycollection) 100.0 3000.0 "RIF_Constant" true 500001.0))

(fn `UserConstructionScript`)